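; Linked portal-pair actor that renders each portal's view through the other and places either portal on valid surfaces.
; Each tick, scene captures follow the player camera relative to the portals, feeding clip-planed views into viewport-scaled render targets.
; Placement nudges a dummy portal until four edge traces hit the allowed surface type, then scales the portal up.
; Overlap events are empty, leaving Blueprint teleport logic unconnected; a comment points to Visual Studio.
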(event `self.ReceiveBeginPlay`
  (`self.SetTickGroup` "TG_PrePhysics")
  (`|ExecutionSequence`
    (:`then_0`
      (bind _output_get (set `self.PortalRT1` "/Game/BP/Portal/RT_P1.RT_P1"))
      (set `SceneCaptureComponent2D.TextureTarget` _output_get (`self.P2Capture`)))
    (:`then_1`
      (bind _output_get_2 (set `self.PortalRT2` "/Game/BP/Portal/RT_P2.RT_P2"))
      (set `SceneCaptureComponent2D.TextureTarget` _output_get_2 (`self.P1Capture`))
      (`self.SetClipPlanes`))))

(event `self.ReceiveTick`
  (params (DeltaSeconds :type "Float (single-precision)"))
  (`SceneComponent.K2_SetWorldLocation` (`self.PSim_D2`) (`PlayerCameraManager.GetCameraLocation` (`GameplayStatics.GetPlayerCameraManager` 0)) false false)
  (`SceneComponent.K2_SetWorldLocation` (`self.PSim_D1`) (`PlayerCameraManager.GetCameraLocation` (`GameplayStatics.GetPlayerCameraManager` 0)) false false)
  (`self.UpdateCamerasD2`)
  (`self.UpdateCaptureM` (`self.P1Capture`) (`self.PSim_D2`))
  (`self.UpdateCamerasD1`)
  (`self.UpdateCaptureM` (`self.P2Capture`) (`self.PSim_D1`))
  (`self.CheckResolution`))

(event `self.Col2.OnComponentBeginOverlap`
  (params (OverlappedComponent :type "PrimitiveComponent Object Reference") (OtherActor :type "Actor Object Reference") (OtherComp :type "PrimitiveComponent Object Reference") (OtherBodyIndex :type Integer) (bFromSweep :type Boolean) (SweepResult :type "HitResult Structure (by ref)"))
  ; Wprowadzone w VisualStudio
)

(event `self.Col1.OnComponentBeginOverlap`
  (params (OverlappedComponent :type "PrimitiveComponent Object Reference") (OtherActor :type "Actor Object Reference") (OtherComp :type "PrimitiveComponent Object Reference") (OtherBodyIndex :type Integer) (bFromSweep :type Boolean) (SweepResult :type "HitResult Structure (by ref)"))
  ; Wprowadzone w VisualStudio
)

(event `self.Col2.OnComponentEndOverlap`
  (params (OverlappedComponent :type "PrimitiveComponent Object Reference") (OtherActor :type "Actor Object Reference") (OtherComp :type "PrimitiveComponent Object Reference") (OtherBodyIndex :type Integer))
  ; Wprowadzone w VisualStudio
)

(event `self.Col1.OnComponentEndOverlap`
  (params (OverlappedComponent :type "PrimitiveComponent Object Reference") (OtherActor :type "Actor Object Reference") (OtherComp :type "PrimitiveComponent Object Reference") (OtherBodyIndex :type Integer))
  ; Wprowadzone w VisualStudio
)

(event `PlacePortal`
  (params (`Blue/Orange` :type Boolean) (NewLocation :type "Vector Structure") (NewRotation :type "Rotator Structure"))
  (bind _returnvalue (select `bool` `Blue/Orange` :`false` (`self.D2`) :`true` (`self.D1`)))
  (`self.CanPlacePortal` NewLocation NewRotation
    (:`CanPlace`
      (`SceneComponent.SetRelativeScale3D` _returnvalue (0.1 0.1 0.1))
      (`SceneComponent.K2_SetWorldLocationAndRotation` _returnvalue (`SceneComponent.K2_GetComponentLocation` (`self.DummyPortal`)) NewRotation false false)
      (bind (_direction _scale) (`Timeline|ScaleUp` :!via `PlayFromStart`)
        (:`Update`
          (`SceneComponent.SetRelativeScale3D` _returnvalue (`KismetMathLibrary.Conv_DoubleToVector` _scale)))))))

(fn `CheckResolution`
  (bind (_returnvalue_x _returnvalue_y) (`KismetMathLibrary.BreakVector2D` (`WidgetLayoutLibrary.GetViewportSize`)))
  (bind (_returnvalue_x_2 _returnvalue_y_2) (`KismetMathLibrary.BreakVector2D` (`WidgetLayoutLibrary.GetViewportSize`)))
  (bind _portalrt2 (`self.PortalRT2`))
  (bind _portalquality (`self.PortalQuality`))
  (bind _portalquality_2 (`self.PortalQuality`))
  (bind _portalrt1 (`self.PortalRT1`))
  (bind _returnvalue (`KismetMathLibrary.FTrunc` (* _returnvalue_y_2 _portalquality_2)))
  (bind _returnvalue_2 (`KismetMathLibrary.FTrunc` (* _returnvalue_x _portalquality)))
  (bind _returnvalue_3 (`KismetMathLibrary.FTrunc` (* _returnvalue_y _portalquality)))
  (bind _returnvalue_4 (`KismetMathLibrary.FTrunc` (* _returnvalue_x_2 _portalquality_2)))
  (`|ExecutionSequence`
    (:`then_0`
      (if (not (and (== _returnvalue_4 (`TextureRenderTarget2D.SizeX` _portalrt1)) (== _returnvalue (`TextureRenderTarget2D.SizeY` _portalrt1))))
        (`KismetRenderingLibrary.ResizeRenderTarget2D` (`self.PortalRT1`) _returnvalue_4 _returnvalue)))
    (:`then_1`
      (if (not (and (== _returnvalue_2 (`TextureRenderTarget2D.SizeX` _portalrt2)) (== _returnvalue_3 (`TextureRenderTarget2D.SizeY` _portalrt2))))
        (`KismetRenderingLibrary.ResizeRenderTarget2D` (`self.PortalRT2`) _returnvalue_2 _returnvalue_3)))))

(fn `CheckSurface`
  (params (InputPin :type "SceneComponent Object Reference"))
  (returns (ReturnValue :type Boolean))
  (bind _returnvalue (`SceneComponent.K2_GetComponentLocation` InputPin))
  (bind (_outhit _returnvalue_2) (`KismetSystemLibrary.LineTraceSingle` _returnvalue (+ _returnvalue (* (`SceneComponent.GetForwardVector` InputPin) 50.0)) "TraceTypeQuery1"))
  (if _returnvalue_2
    (return (`|EnumEquality` (`PhysicalMaterial.SurfaceType` (`.PhysMat` (`GameplayStatics.BreakHitResult` _outhit))) "SurfaceType1"))
    (else
      (return false))))

(fn `GetCamRoot1Comp`
  (returns (ReturnValue :type "SceneComponent Object Reference"))
  (return (`self.CamRoot1`)))

(fn `GetCamRoot2Comp`
  (returns (ReturnValue :type "SceneComponent Object Reference"))
  (return (`self.CamRoot2`)))

(fn `GetCol1Comp`
  (returns (ReturnValue :type "BoxComponent Object Reference"))
  (return (`self.Col1`)))

(fn `GetCol2Comp`
  (returns (ReturnValue :type "BoxComponent Object Reference"))
  (return (`self.Col2`)))

(fn `GetD1Comp`
  (returns (ReturnValue :type "SceneComponent Object Reference"))
  (return (`self.D1`)))

(fn `GetD1ForwardDirectionComp`
  (returns (ReturnValue :type "ArrowComponent Object Reference"))
  (return (`self.Arrow`)))

(fn `GetD2Comp`
  (returns (ReturnValue :type "SceneComponent Object Reference"))
  (return (`self.D2`)))

(fn `GetD2ForwardDirectionComp`
  (returns (ReturnValue :type "ArrowComponent Object Reference"))
  (return (`self.Arrow1`)))

(fn `GetDComp`
  (returns (ReturnValue :type "SceneComponent Object Reference"))
  (return (`self.D`)))

(fn `GetDoor1Comp`
  (returns (ReturnValue :type "StaticMeshComponent Object Reference"))
  (return (`self.Door1`)))

(fn `GetDoor2Comp`
  (returns (ReturnValue :type "StaticMeshComponent Object Reference"))
  (return (`self.Door2`)))

(fn `GetDummyPortalComp`
  (returns (ReturnValue :type "SceneComponent Object Reference"))
  (return (`self.DummyPortal`)))

(fn `GetExitCollider`
  (returns (ReturnValue :type "BoxComponent Object Reference"))
  (return (`self.ExitColider`)))

(fn `GetLComp`
  (returns (ReturnValue :type "SceneComponent Object Reference"))
  (return (`self.L`)))

(fn `GetP1CaptureComp`
  (returns (ReturnValue :type "SceneCaptureComponent2D Object Reference"))
  (return (`self.P1Capture`)))

(fn `GetP2CaptureComp`
  (returns (ReturnValue :type "SceneCaptureComponent2D Object Reference"))
  (return (`self.P2Capture`)))

(fn `GetPSim_D1Comp`
  (returns (ReturnValue :type "SceneComponent Object Reference"))
  (return (`self.PSim_D1`)))

(fn `GetPSim_D2Comp`
  (returns (ReturnValue :type "SceneComponent Object Reference"))
  (return (`self.PSim_D2`)))

(fn `GetRComp`
  (returns (ReturnValue :type "SceneComponent Object Reference"))
  (return (`self.R`)))

(fn `GetTargetPoint`
  (params (SweepResult :type "HitResult Structure") (TP_Enter :type "SceneComponent Object Reference") (TP_Exit :type "SceneComponent Object Reference"))
  (returns (NewParam1 :type "Vector Structure"))
  (`SceneComponent.K2_SetWorldLocation` TP_Enter (`.ImpactPoint` (`GameplayStatics.BreakHitResult` SweepResult)) false false)
  (`SceneComponent.K2_SetRelativeLocation` TP_Exit (* (`SceneComponent.RelativeLocation` TP_Enter) (1.0 -1.0 1.0)) false false)
  (return (`SceneComponent.K2_GetComponentLocation` TP_Exit)))

(fn `GetTP1Comp`
  (returns (ReturnValue :type "SceneComponent Object Reference"))
  (return (`self.TP1`)))

(fn `GetTP2Comp`
  (returns (ReturnValue :type "SceneComponent Object Reference"))
  (return (`self.TP2`)))

(fn `GetUComp`
  (returns (ReturnValue :type "SceneComponent Object Reference"))
  (return (`self.U`)))

(fn `SetClipPlanes`
  (bind _p2capture (`self.P2Capture`))
  (bind _p1capture (`self.P1Capture`))
  (`|ExecutionSequence`
    (:`then_0`
      (set `SceneCaptureComponent2D.bEnableClipPlane` true _p1capture)
      (set `SceneCaptureComponent2D.ClipPlaneBase` (+ (`SceneComponent.K2_GetComponentLocation` _p1capture) (* (`SceneComponent.GetForwardVector` (`self.Arrow`)) -10.0)) _p1capture)
      (set `SceneCaptureComponent2D.ClipPlaneNormal` (`SceneComponent.GetForwardVector` (`self.Arrow`)) _p1capture))
    (:`then_1`
      (set `SceneCaptureComponent2D.bEnableClipPlane` true _p2capture)
      (set `SceneCaptureComponent2D.ClipPlaneBase` (+ (`SceneComponent.K2_GetComponentLocation` _p2capture) (* (`SceneComponent.GetForwardVector` (`self.Arrow1`)) -10.0)) _p2capture)
      (set `SceneCaptureComponent2D.ClipPlaneNormal` (`SceneComponent.GetForwardVector` (`self.Arrow1`)) _p2capture))))

(fn `UpdateCamerasD1`
  (bind _returnvalue (`SceneComponent.K2_GetComponentToWorld` (`self.D2`)))
  (bind _returnvalue_2 (`SceneComponent.K2_GetComponentToWorld` (`self.D1`)))
  (bind (_x _y _z) (`KismetMathLibrary.BreakRotIntoAxes` (`SceneComponent.K2_GetComponentRotation` (`PlayerCameraManager.TransformComponent` (`GameplayStatics.GetPlayerCameraManager` 0)))))
  (`/Engine/EditorBlueprintResources/StandardMacros.IsValid` (`self.P2Capture`)
    (:`Is Valid`
      (`SceneComponent.K2_SetWorldLocationAndRotation` (`self.P2Capture`) (`KismetMathLibrary.TransformLocation` (`SceneComponent.K2_GetComponentToWorld` (`self.D2`)) (`KismetMathLibrary.InverseTransformLocation` (`KismetMathLibrary.MakeTransform` (.location (`SceneComponent.K2_GetComponentToWorld` (`self.D1`))) (.rotation (`SceneComponent.K2_GetComponentToWorld` (`self.D1`))) (`KismetMathLibrary.MakeVector` (* (.x (.scale (`SceneComponent.K2_GetComponentToWorld` (`self.D1`)))) -1.0) (* (.y (.scale (`SceneComponent.K2_GetComponentToWorld` (`self.D1`)))) -1.0) (.z (.scale (`SceneComponent.K2_GetComponentToWorld` (`self.D1`)))))) (`SceneComponent.K2_GetComponentLocation` (`PlayerCameraManager.TransformComponent` (`GameplayStatics.GetPlayerCameraManager` 0))))) (`KismetMathLibrary.MakeRotationFromAxes` (`KismetMathLibrary.TransformDirection` _returnvalue (`KismetMathLibrary.MirrorVectorByNormal` (`KismetMathLibrary.MirrorVectorByNormal` (`KismetMathLibrary.InverseTransformDirection` _returnvalue_2 _x) (1.0 0.0 0.0)) (0.0 1.0 0.0))) (`KismetMathLibrary.TransformDirection` _returnvalue (`KismetMathLibrary.MirrorVectorByNormal` (`KismetMathLibrary.MirrorVectorByNormal` (`KismetMathLibrary.InverseTransformDirection` _returnvalue_2 _y) (1.0 0.0 0.0)) (0.0 1.0 0.0))) (`KismetMathLibrary.TransformDirection` _returnvalue (`KismetMathLibrary.MirrorVectorByNormal` (`KismetMathLibrary.MirrorVectorByNormal` (`KismetMathLibrary.InverseTransformDirection` _returnvalue_2 _z) (1.0 0.0 0.0)) (0.0 1.0 0.0)))) false false))))

(fn `UpdateCamerasD2`
  (bind _returnvalue (`SceneComponent.K2_GetComponentToWorld` (`self.D1`)))
  (bind _returnvalue_2 (`SceneComponent.K2_GetComponentToWorld` (`self.D2`)))
  (bind (_x _y _z) (`KismetMathLibrary.BreakRotIntoAxes` (`SceneComponent.K2_GetComponentRotation` (`PlayerCameraManager.TransformComponent` (`GameplayStatics.GetPlayerCameraManager` 0)))))
  (`/Engine/EditorBlueprintResources/StandardMacros.IsValid` (`self.P1Capture`)
    (:`Is Valid`
      (`SceneComponent.K2_SetWorldLocationAndRotation` (`self.P1Capture`) (`KismetMathLibrary.TransformLocation` (`SceneComponent.K2_GetComponentToWorld` (`self.D1`)) (`KismetMathLibrary.InverseTransformLocation` (`KismetMathLibrary.MakeTransform` (.location (`SceneComponent.K2_GetComponentToWorld` (`self.D2`))) (.rotation (`SceneComponent.K2_GetComponentToWorld` (`self.D2`))) (`KismetMathLibrary.MakeVector` (* (.x (.scale (`SceneComponent.K2_GetComponentToWorld` (`self.D2`)))) -1.0) (* (.y (.scale (`SceneComponent.K2_GetComponentToWorld` (`self.D2`)))) -1.0) (.z (.scale (`SceneComponent.K2_GetComponentToWorld` (`self.D2`)))))) (`SceneComponent.K2_GetComponentLocation` (`PlayerCameraManager.TransformComponent` (`GameplayStatics.GetPlayerCameraManager` 0))))) (`KismetMathLibrary.MakeRotationFromAxes` (`KismetMathLibrary.TransformDirection` _returnvalue (`KismetMathLibrary.MirrorVectorByNormal` (`KismetMathLibrary.MirrorVectorByNormal` (`KismetMathLibrary.InverseTransformDirection` _returnvalue_2 _x) (1.0 0.0 0.0)) (0.0 1.0 0.0))) (`KismetMathLibrary.TransformDirection` _returnvalue (`KismetMathLibrary.MirrorVectorByNormal` (`KismetMathLibrary.MirrorVectorByNormal` (`KismetMathLibrary.InverseTransformDirection` _returnvalue_2 _y) (1.0 0.0 0.0)) (0.0 1.0 0.0))) (`KismetMathLibrary.TransformDirection` _returnvalue (`KismetMathLibrary.MirrorVectorByNormal` (`KismetMathLibrary.MirrorVectorByNormal` (`KismetMathLibrary.InverseTransformDirection` _returnvalue_2 _z) (1.0 0.0 0.0)) (0.0 1.0 0.0)))) false false))))

(fn `UserConstructionScript`)