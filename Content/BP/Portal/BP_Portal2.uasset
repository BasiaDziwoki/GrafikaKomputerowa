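; Portal actor holding a linked blue/orange portal pair, with live view captures and surface-checked placement.
; Each tick mirrors the player camera through simulated points to aim both scene captures, narrowing FOV with distance.
; Placement nudges a dummy portal until four edge traces hit the allowed physical surface, then moves and scales up the chosen portal.
; Blueprint teleport logic is disconnected, noted as moved to Visual Studio, with component getters exposed.
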(event `self.ReceiveTick`
  (params (DeltaSeconds :type "Float (single-precision)"))
  (`self.UpdateCameras`))

(event `self.Col2.OnComponentBeginOverlap`
  (params (OverlappedComponent :type "PrimitiveComponent Object Reference") (OtherActor :type "Actor Object Reference") (OtherComp :type "PrimitiveComponent Object Reference") (OtherBodyIndex :type Integer) (bFromSweep :type Boolean) (SweepResult :type "HitResult Structure (by ref)"))
  ; Wprowadzone w VisualStudio
)

(event `self.Col1.OnComponentBeginOverlap`
  (params (OverlappedComponent :type "PrimitiveComponent Object Reference") (OtherActor :type "Actor Object Reference") (OtherComp :type "PrimitiveComponent Object Reference") (OtherBodyIndex :type Integer) (bFromSweep :type Boolean) (SweepResult :type "HitResult Structure (by ref)"))
  ; Wprowadzone w VisualStudio
)

(event `self.Col2.OnComponentEndOverlap`
  (params (OverlappedComponent :type "PrimitiveComponent Object Reference") (OtherActor :type "Actor Object Reference") (OtherComp :type "PrimitiveComponent Object Reference") (OtherBodyIndex :type Integer))
  ; Wprowadzone w VisualStudio
)

(event `self.Col1.OnComponentEndOverlap`
  (params (OverlappedComponent :type "PrimitiveComponent Object Reference") (OtherActor :type "Actor Object Reference") (OtherComp :type "PrimitiveComponent Object Reference") (OtherBodyIndex :type Integer))
  ; Wprowadzone w VisualStudio
)

(event `PlacePortal`
  (params (`Blue/Orange` :type Boolean) (NewLocation :type "Vector Structure") (NewRotation :type "Rotator Structure"))
  (bind _returnvalue (select `bool` `Blue/Orange` :`false` (`self.D2`) :`true` (`self.D1`)))
  (`self.CanPlacePortal` NewLocation NewRotation
    (:`CanPlace`
      (`SceneComponent.SetRelativeScale3D` _returnvalue (0.1 0.1 0.1))
      (`SceneComponent.K2_SetWorldLocationAndRotation` _returnvalue (`SceneComponent.K2_GetComponentLocation` (`self.DummyPortal`)) NewRotation false false)
      (bind (_direction _scale) (`Timeline|ScaleUp` :!via `PlayFromStart`)
        (:`Update`
          (`SceneComponent.SetRelativeScale3D` _returnvalue (`KismetMathLibrary.Conv_DoubleToVector` _scale)))))))

(fn `CheckSurface`
  (params (InputPin :type "SceneComponent Object Reference"))
  (returns (ReturnValue :type Boolean))
  (bind _returnvalue (`SceneComponent.K2_GetComponentLocation` InputPin))
  (bind (_outhit _returnvalue_2) (`KismetSystemLibrary.LineTraceSingle` _returnvalue (+ _returnvalue (* (`SceneComponent.GetForwardVector` InputPin) 50.0)) "TraceTypeQuery1"))
  (if _returnvalue_2
    (return (`|EnumEquality` (`PhysicalMaterial.SurfaceType` (`.PhysMat` (`GameplayStatics.BreakHitResult` _outhit))) "SurfaceType1"))
    (else
      (return false))))

(fn `GetCamRoot1Comp`
  (returns (ReturnValue :type "SceneComponent Object Reference"))
  (return (`self.CamRoot1`)))

(fn `GetCamRoot2Comp`
  (returns (ReturnValue :type "SceneComponent Object Reference"))
  (return (`self.CamRoot2`)))

(fn `GetCol1Comp`
  (returns (ReturnValue :type "BoxComponent Object Reference"))
  (return (`self.Col1`)))

(fn `GetCol2Comp`
  (returns (ReturnValue :type "BoxComponent Object Reference"))
  (return (`self.Col2`)))

(fn `GetD1Comp`
  (returns (ReturnValue :type "SceneComponent Object Reference"))
  (return (`self.D1`)))

(fn `GetD1ForwardDirectionComp`
  (returns (ReturnValue :type "ArrowComponent Object Reference"))
  (return (`self.Arrow`)))

(fn `GetD2Comp`
  (returns (ReturnValue :type "SceneComponent Object Reference"))
  (return (`self.D2`)))

(fn `GetD2ForwardDirectionComp`
  (returns (ReturnValue :type "ArrowComponent Object Reference"))
  (return (`self.Arrow1`)))

(fn `GetDComp`
  (returns (ReturnValue :type "SceneComponent Object Reference"))
  (return (`self.D`)))

(fn `GetDoor1Comp`
  (returns (ReturnValue :type "StaticMeshComponent Object Reference"))
  (return (`self.Door1`)))

(fn `GetDoor2Comp`
  (returns (ReturnValue :type "StaticMeshComponent Object Reference"))
  (return (`self.Door2`)))

(fn `GetDummyPortalComp`
  (returns (ReturnValue :type "SceneComponent Object Reference"))
  (return (`self.DummyPortal`)))

(fn `GetExitCollider`
  (returns (ReturnValue :type "BoxComponent Object Reference"))
  (return (`self.ExitColider`)))

(fn `GetLComp`
  (returns (ReturnValue :type "SceneComponent Object Reference"))
  (return (`self.L`)))

(fn `GetP1CaptureComp`
  (returns (ReturnValue :type "SceneCaptureComponent2D Object Reference"))
  (return (`self.P1Capture`)))

(fn `GetP2CaptureComp`
  (returns (ReturnValue :type "SceneCaptureComponent2D Object Reference"))
  (return (`self.P2Capture`)))

(fn `GetPSim_D1Comp`
  (returns (ReturnValue :type "SceneComponent Object Reference"))
  (return (`self.PSim_D1`)))

(fn `GetPSim_D2Comp`
  (returns (ReturnValue :type "SceneComponent Object Reference"))
  (return (`self.PSim_D2`)))

(fn `GetRComp`
  (returns (ReturnValue :type "SceneComponent Object Reference"))
  (return (`self.R`)))

(fn `GetTargetPoint`
  (params (SweepResult :type "HitResult Structure") (TP_Enter :type "SceneComponent Object Reference") (TP_Exit :type "SceneComponent Object Reference"))
  (returns (NewParam1 :type "Vector Structure"))
  (`SceneComponent.K2_SetWorldLocation` TP_Enter (`.ImpactPoint` (`GameplayStatics.BreakHitResult` SweepResult)) false false)
  (`SceneComponent.K2_SetRelativeLocation` TP_Exit (* (`SceneComponent.RelativeLocation` TP_Enter) (1.0 -1.0 1.0)) false false)
  (return (`SceneComponent.K2_GetComponentLocation` TP_Exit)))

(fn `GetTP1Comp`
  (returns (ReturnValue :type "SceneComponent Object Reference"))
  (return (`self.TP1`)))

(fn `GetTP2Comp`
  (returns (ReturnValue :type "SceneComponent Object Reference"))
  (return (`self.TP2`)))

(fn `GetUComp`
  (returns (ReturnValue :type "SceneComponent Object Reference"))
  (return (`self.U`)))

(fn `UpdateCameras`
  (`SceneComponent.K2_SetWorldLocation` (`self.PSim_D1`) (`PlayerCameraManager.GetCameraLocation` (`GameplayStatics.GetPlayerCameraManager` 0)) false false)
  (`SceneComponent.K2_SetWorldLocation` (`self.PSim_D2`) (`PlayerCameraManager.GetCameraLocation` (`GameplayStatics.GetPlayerCameraManager` 0)) false false)
  (`self.UpdateCaptureM` (`self.P1Capture`) (`self.PSim_D2`))
  (`self.UpdateCaptureM` (`self.P2Capture`) (`self.PSim_D1`))
  (return))

(fn `UserConstructionScript`)