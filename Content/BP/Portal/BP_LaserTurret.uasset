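; Portal laser turret that draws a Niagara beam and drains the player's health through a capsule hit volume.
; Each Tick damages the overlapping player, using the last begin-overlap actor, and refreshes beam endpoints through functions defined outside this graph.
; AnyDamage calls a same-named function and stops the health drain.
; Getters expose components and timelines; the local side-panel animation, trace and shutdown nodes are disconnected.
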(event `self.ReceiveBeginPlay`
  (bind _ns_beam (`self.NS_Beam`))
  (bind _returnvalue (`SceneComponent.K2_GetComponentLocation` (`self.Cube`)))
  (set `self.isCapsuleExisting` true)
  (`NiagaraComponent.SetVariableVec3` _ns_beam "User.BeamStart" _returnvalue)
  (`NiagaraComponent.SetVariableVec3` _ns_beam "User.Beam End" (* _returnvalue (-20.0 1.0 1.0))))

(event `self.ReceiveTick`
  (params (DeltaSeconds :type "Float (single-precision)"))
  (`|ExecutionSequence`
    (:`then_0`
      (if (`self.isCapsuleExisting`)
        (if (`PrimitiveComponent.IsOverlappingActor` (`self.Capsule`) (`GameplayStatics.GetPlayerCharacter` 0))
          (bind _asbp_first_person_character (cast `/Game/FirstPerson/Blueprints/BP_FirstPersonCharacter` (stale `self.Capsule.OnComponentBeginOverlap` OtherActor)))
          (`/Game/FirstPerson/Blueprints/BP_FirstPersonCharacter.LosingHealth` _asbp_first_person_character 1.0))))
    (:`then_1`
      (`self.ChangeLaserEndingLocation`))
    (:`then_2`
      (`self.ChangeLaserBeginLocation`))))

(event `self.Capsule.OnComponentBeginOverlap`
  (params (OverlappedComponent :type "PrimitiveComponent Object Reference") (OtherActor :type "Actor Object Reference") (OtherComp :type "PrimitiveComponent Object Reference") (OtherBodyIndex :type Integer) (bFromSweep :type Boolean) (SweepResult :type "HitResult Structure (by ref)")))

(event `self.ReceiveAnyDamage`
  (params (Damage :type "Float (single-precision)") (DamageType :type "DamageType Object Reference") (InstigatedBy :type "Controller Object Reference") (DamageCauser :type "Actor Object Reference"))
  (`self.AnyDamage`)
  (set `self.isCapsuleExisting` false))

(fn `GetCapsuleComp`
  (returns (ReturnValue :type "CapsuleComponent Object Reference"))
  (return (`self.Capsule`)))

(fn `GetCubeComp`
  (returns (ReturnValue :type "StaticMeshComponent Object Reference"))
  (return (`self.Cube`)))

(fn `GetLaserComp`
  (returns (ReturnValue :type "NiagaraComponent Object Reference"))
  (return (`self.NS_Beam`)))

(fn `GetTurretBaseComp`
  (returns (ReturnValue :type "StaticMeshComponent Object Reference"))
  (return (`self.TurretBase`)))

(fn `GetTurretLeftComp`
  (returns (ReturnValue :type "StaticMeshComponent Object Reference"))
  (return (`self.TurretLeft`)))

(fn `GetTurretLeftPositionTimeline`
  (returns (ReturnValue :type "TimelineComponent Object Reference"))
  (return (`self.TurretLeftPosition`)))

(fn `GetTurretRightComp`
  (returns (ReturnValue :type "StaticMeshComponent Object Reference"))
  (return (`self.TurretRight`)))

(fn `GetTurretRightPositionTimeline`
  (returns (ReturnValue :type "TimelineComponent Object Reference"))
  (return (`self.TurretRightPosition`)))

(fn `UserConstructionScript`)