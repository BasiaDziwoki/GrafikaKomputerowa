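; BP_Door is a two-panel sliding door that opens when enough pressure switches are active.
; SwitchActivated and SwitchDeactivated events raise or lower an active-switch count and compare it to a required count.
; Meeting the threshold plays left and right timelines that set each mesh's relative Y location; falling short reverses them.
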(event `SwitchActivated`
  (`/Engine/EditorBlueprintResources/StandardMacros.IncrementInt` (`self.PressureSwitchesActive`)
    (:`  `
      (if (>= (`self.PressureSwitchesActive`) (`self.PressureSwitchesNeeded`))
        (`|ExecutionSequence`
          (:`then_0`
            (bind (_direction _doorrightposition) (`Timeline|DoorRightActivation` :!label _label)
              (:`Update`
                (`SceneComponent.K2_SetRelativeLocation` (`self.DoorRightMesh`) (`KismetMathLibrary.MakeVector` 0.0 _doorrightposition) false false))))
          (:`then_1`
            (bind (_direction_2 _doorleftposition) (`Timeline|DoorLeftActivation` :!label _label_2)
              (:`Update`
                (`SceneComponent.K2_SetRelativeLocation` (`self.DoorLeftMesh`) (`KismetMathLibrary.MakeVector` 0.0 _doorleftposition) false false)))))
        (else
          (`|ExecutionSequence`
            (:`then_0`
              (goto _label :!via `Reverse`))
            (:`then_1`
              (goto _label_2 :!via `Reverse`))))))))

(event `SwitchDeactivated`
  (`/Engine/EditorBlueprintResources/StandardMacros.DecrementInt` (`self.PressureSwitchesActive`)
    (:`  `
      (if (>= (`self.PressureSwitchesActive`) (`self.PressureSwitchesNeeded`))
        (`|ExecutionSequence`
          (:`then_0`
            (goto _label))
          (:`then_1`
            (goto _label_2)))
        (else
          (`|ExecutionSequence`
            (:`then_0`
              (goto _label :!via `Reverse`))
            (:`then_1`
              (goto _label_2 :!via `Reverse`))))))))

(fn `UserConstructionScript`)